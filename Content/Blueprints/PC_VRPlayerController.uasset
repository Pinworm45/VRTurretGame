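; PC_VRPlayerController is a player controller that switches the player's possession between a BaseShip and its mounted turrets.
; BeginPlay caches the starting pawn as PlayerShip, whose TurretArray child actors serve as possessable BaseTurrets.
; Number keys select the first two turrets, and pressing the active one's key returns control to the ship via UnpossesTurrets.
; Next and Previous inputs step through turrets, using a failed cast to wrap around the array.
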(event `self.ReceiveBeginPlay`
  ;[1 1 1] Begin Play, set player ship, enable input
  (bind _asbase_ship (cast `/Game/Blueprints/Ships/BaseShip` (`GameplayStatics.GetPlayerPawn` 0)))
  (set `self.PlayerShip` _asbase_ship)
  (`self.EnableInput` (`GameplayStatics.GetPlayerController` 0)))

(event `Key|One`
  (params (Key :type "Key Structure" :default "AnyKey"))
  (bind _activeturret (`self.ActiveTurret`))
  (bind (_asbase_turret _bsuccess) (cast `/Game/Blueprints/Turrets/BaseTurret` (`ChildActorComponent.ChildActor` (`KismetArrayLibrary.Array_Get` (`/Game/Blueprints/Ships/BaseShip.TurretArray` (`self.PlayerShip`)) _activeturret)) :!pure true))
  ;[1 1 1] Select Specific Turrets
  (:`Pressed`
    (if (!= _activeturret 0)
      (set `self.ActiveTurret` 0)
      (if _bsuccess
        (`self.Possess` _asbase_turret))
      (else
        (`self.UnpossesTurrets`)))))

(event `Key|Two`
  (params (Key :type "Key Structure" :default "AnyKey"))
  (bind _activeturret (`self.ActiveTurret`))
  (bind (_asbase_turret _bsuccess) (cast `/Game/Blueprints/Turrets/BaseTurret` (`ChildActorComponent.ChildActor` (`KismetArrayLibrary.Array_Get` (`/Game/Blueprints/Ships/BaseShip.TurretArray` (`self.PlayerShip`)) _activeturret)) :!pure true))
  ;[1 1 1] Select Specific Turrets
  (:`Pressed`
    (if (!= _activeturret 1)
      (set `self.ActiveTurret` 1)
      (if _bsuccess
        (`self.Possess` _asbase_turret))
      (else
        (`self.UnpossesTurrets`)))))

(event `InputAction|NextTurret`
  (params (Key :type "Key Structure" :default "AnyKey"))
  (bind _turretarray (`/Game/Blueprints/Ships/BaseShip.TurretArray` (`self.PlayerShip`)))
  ;[1 1 1] Next Turret
  (:`Pressed`
    (bind _result (`/Engine/EditorBlueprintResources/StandardMacros.IncrementInt` (`self.ActiveTurret`))
      (:`  `
        (bind (_asbase_turret _bsuccess) (cast `/Game/Blueprints/Turrets/BaseTurret` (`ChildActorComponent.ChildActor` (`KismetArrayLibrary.Array_Get` _turretarray _result)) :!pure true))
        (if _bsuccess
          (`self.Possess` _asbase_turret)
          (else
            (`self.Possess` (cast `/Game/Blueprints/Turrets/BaseTurret` (`ChildActorComponent.ChildActor` (`KismetArrayLibrary.Array_Get` _turretarray)) :!pure true))
            (set `self.ActiveTurret` 0)))))))

(event `InputAction|PreviousTurret`
  (params (Key :type "Key Structure" :default "AnyKey"))
  (bind _turretarray (`/Game/Blueprints/Ships/BaseShip.TurretArray` (`self.PlayerShip`)))
  (bind _returnvalue (`KismetArrayLibrary.Array_LastIndex` _turretarray))
  ;[1 1 1] Previous Turret
  (:`Pressed`
    (bind _result (`/Engine/EditorBlueprintResources/StandardMacros.DecrementInt` (`self.ActiveTurret`))
      (:`  `
        (bind (_asbase_turret _bsuccess) (cast `/Game/Blueprints/Turrets/BaseTurret` (`ChildActorComponent.ChildActor` (`KismetArrayLibrary.Array_Get` _turretarray _result)) :!pure true))
        (if _bsuccess
          (`self.Possess` _asbase_turret)
          (else
            (`self.Possess` (cast `/Game/Blueprints/Turrets/BaseTurret` (`ChildActorComponent.ChildActor` (`KismetArrayLibrary.Array_Get` _turretarray _returnvalue)) :!pure true))
            (set `self.ActiveTurret` _returnvalue)))))))

(fn `UnpossesTurrets`
  (`self.UnPossess` (`GameplayStatics.GetPlayerController` 0))
  (`self.Possess` (`self.PlayerShip`))
  (set `self.ActiveTurret` -1))

(fn `UserConstructionScript`)