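; BaseEnemy is an enemy actor that wanders in random directions and can be killed.
; It picks a random rotation on BeginPlay and on a looping timer, while Tick pushes it along local forward by ForwardSpeed, without sweep or delta-time scaling.
; ApplyDamage subtracts from Health and, at zero or below, spawns DM_UFO at the static mesh's transform and destroys the actor.
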(event `self.ReceiveBeginPlay`
  (`KismetSystemLibrary.K2_SetTimerDelegate` (delegate `RandomRot`) 10.0 true)
  (`self.K2_SetActorRotation` (`KismetMathLibrary.RandomRotator` false) :!label _label))

(event `RandomRot`
  (goto _label))

(event `self.ReceiveTick`
  (params (DeltaSeconds :type "Float (single-precision)"))
  (`self.K2_AddActorLocalOffset` (`KismetMathLibrary.MakeVector` (`self.ForwardSpeed`))))

(fn `ApplyDamage`
  (params (Damage :type "Float (double-precision)"))
  (bind _output_get (set `self.Health` (- (`self.Health`) Damage)))
  (if (<= _output_get 0.0)
    (`|SpawnActorFromClass` "/Game/Blueprints/Enemies/DM_UFO.DM_UFO_C" (`SceneComponent.K2_GetComponentToWorld` (`self.StaticMesh`)) "Undefined" "OverrideRootScale")
    (`self.K2_DestroyActor`)))

(fn `UserConstructionScript`)