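; Possessable player turret that rotates its mesh with look input and fires bullets and homing-target missiles.
; While possessed, Tick traces along the fire arrow to set Target, plus along camera forward in VR to set VRTarget, accepting EnemyTargetable actors.
; Held fire opens a gate for delay-limited bullets aimed at Target, or straight ahead without one.
; Alt fire launches missiles at VRTarget, falling back to Target, with a short cooldown.
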(event `InputAxis|LookUp`
  (params (AxisValue :type "Float (single-precision)"))
  ;[1 1 1] Rotation
  (if (!= AxisValue 0.0)
    (`SceneComponent.K2_AddRelativeRotation` (`self.StaticMesh`) (`KismetMathLibrary.MakeRotator` (* AxisValue 2.0)) false false)))

(event `InputAxis|LookRight`
  (params (AxisValue :type "Float (single-precision)"))
  ;[1 1 1] Rotation
  (if (!= AxisValue 0.0)
    (`SceneComponent.K2_AddRelativeRotation` (`self.StaticMesh`) (`KismetMathLibrary.MakeRotator` 0.0 0.0 (* AxisValue 2.0)) false false)))

(event `InputAction|AltFire`
  (params (Key :type "Key Structure" :default "AnyKey"))
  (bind _firearrow (`self.FireArrow`))
  (bind _vrtarget (`self.VRTarget`))
  (bind _returnvalue (`KismetMathLibrary.MakeTransform` (`SceneComponent.K2_GetComponentLocation` _firearrow) (`SceneComponent.K2_GetComponentRotation` _firearrow)))
  ;[1 1 1] MissileLaunch
  (:`Pressed`
    (if (`self.CanFireMissile`)
      (if (> (`self.Missiles`) 0)
        (set `self.CanFireMissile` false)
        (if (`KismetSystemLibrary.IsValid` _vrtarget)
          (`|SpawnActorFromClass` "/Game/Blueprints/Weapons/Missile.Missile_C" _returnvalue "Undefined" "OverrideRootScale" null 100.0 _vrtarget)
          (`KismetSystemLibrary.Delay` 0.5)
          (set `self.CanFireMissile` true)
          (else
            (`|SpawnActorFromClass` "/Game/Blueprints/Weapons/Missile.Missile_C" _returnvalue "Undefined" "OverrideRootScale" null 100.0 (`self.Target`))
            (`KismetSystemLibrary.Delay` 0.5)
            (set `self.CanFireMissile` true)))))))

(event `self.ReceivePossessed`
  (params (NewController :type "Controller Object Reference"))
  (set `self.Pozzed` true))

(event `self.ReceiveUnpossessed`
  (params (OldController :type "Controller Object Reference"))
  (set `self.Pozzed` false))

(event `self.ReceiveTick`
  (params (DeltaSeconds :type "Float (single-precision)"))
  (bind _firearrow (`self.FireArrow`))
  (bind _target (`self.Target`))
  (bind _vrtarget (`self.VRTarget`))
  (bind _returnvalue (`SceneComponent.K2_GetComponentLocation` (`self.FireArrow`)))
  (bind _returnvalue_2 (`SceneComponent.K2_GetComponentLocation` _firearrow))
  (bind _returnvalue_3 (`SceneComponent.K2_GetComponentLocation` (`self.FireArrow`)))
  ;[1 1 1] Fire Guns
  (if (`self.Pozzed`)
    (`|ExecutionSequence`
      (:`then_0`
        (`/Engine/EditorBlueprintResources/StandardMacros.Gate` true :!label _label
          (:`Exit`
            (if (`self.CanFire`)
              (set `self.CanFire` false)
              (`/Engine/EditorBlueprintResources/StandardMacros.IsValid` _target
                (:`Is Valid`
                  (`|SpawnActorFromClass` "/Game/Blueprints/Weapons/Bullet.Bullet_C" (`KismetMathLibrary.MakeTransform` _returnvalue (`KismetMathLibrary.FindLookAtRotation` _returnvalue (`self.K2_GetActorLocation` _target))) "Undefined" "OverrideRootScale" null 20.0))
                (:`Is Not Valid`
                  (`|SpawnActorFromClass` "/Game/Blueprints/Weapons/Bullet.Bullet_C" (`SceneComponent.K2_GetComponentToWorld` (`self.FireArrow`)) "Undefined" "OverrideRootScale" null 20.0)))
              (`KismetSystemLibrary.Delay` (`self.FireDelay`))
              (set `self.CanFire` true)))))
      (:`then_1`
        (if (`self.Pozzed`)
          (if (`HeadMountedDisplayFunctionLibrary.IsHeadMountedDisplayEnabled`)
            ;[1 1 1] HMD traces
            (`|ExecutionSequence`
              (:`then_0`
                (bind _outhit (`KismetSystemLibrary.LineTraceSingle` :`Start` _returnvalue_3 :`End` (+ _returnvalue_3 (* (`SceneComponent.GetForwardVector` (`PlayerCameraManager.TransformComponent` (`GameplayStatics.GetPlayerCameraManager` 0))) 5000.0)) :`TraceChannel` "TraceTypeQuery1" :`DrawDebugType` "ForOneFrame" :`TraceHitColor` (struct :`G` 1.0)))
                (bind (_bblockinghit _binitialoverlap _time _location _impactpoint _normal _impactnormal _physmat _hitactor) (`GameplayStatics.BreakHitResult` _outhit))
                (if (`KismetSystemLibrary.DoesImplementInterface` _hitactor "/Game/Blueprints/Enemies/EnemyTargetable.EnemyTargetable_C")
                  (`/Engine/EditorBlueprintResources/StandardMacros.IsValid` _vrtarget
                    (:`Is Valid`
                      (if (!= _hitactor _vrtarget)
                        (set `self.VRTarget` _hitactor)
                        (goto _label_2 :!via `Reset`)))
                    (:`Is Not Valid`
                      (set `self.VRTarget` _hitactor)
                      (goto _label_2 :!via `Reset`)))
                  (else
                    (`/Engine/EditorBlueprintResources/StandardMacros.DoOnce` false :!label _label_2
                      (:`Completed`
                        (bind _asbase_enemy (cast `/Game/Blueprints/Enemies/BaseEnemy` (`self.VRTarget`)))
                        (if (not (`KismetSystemLibrary.IsValid` _asbase_enemy))
                          (set `self.VRTarget` null)))))))
              (:`then_1`
                ;[1 1 1] NonVR trace
                (bind _outhit_2 (`KismetSystemLibrary.LineTraceSingle` :`Start` _returnvalue_2 :`End` (+ _returnvalue_2 (* (`SceneComponent.GetForwardVector` _firearrow) 5000.0)) :`TraceChannel` "TraceTypeQuery1" :`DrawDebugType` "ForOneFrame" :!label _label_3))
                (bind (_bblockinghit_2 _binitialoverlap_2 _time_2 _location_2 _impactpoint_2 _normal_2 _impactnormal_2 _physmat_2 _hitactor_2) (`GameplayStatics.BreakHitResult` _outhit_2))
                (if (`KismetSystemLibrary.DoesImplementInterface` _hitactor_2 "/Game/Blueprints/Enemies/EnemyTargetable.EnemyTargetable_C")
                  (`/Engine/EditorBlueprintResources/StandardMacros.IsValid` (`self.Target`)
                    (:`Is Valid`
                      (if (!= _hitactor_2 (`self.Target`))
                        (set `self.Target` _hitactor_2)
                        (goto _label_4 :!via `Reset`)))
                    (:`Is Not Valid`
                      (set `self.Target` _hitactor_2)
                      (goto _label_4 :!via `Reset`)))
                  (else
                    (`/Engine/EditorBlueprintResources/StandardMacros.DoOnce` false :!label _label_4
                      (:`Completed`
                        (bind _asbase_enemy_2 (cast `/Game/Blueprints/Enemies/BaseEnemy` (`self.Target`)))
                        (if (not (`KismetSystemLibrary.IsValid` _asbase_enemy_2))
                          (set `self.Target` null))))))))
            (else
              (goto _label_3))))))))

(event `InputAction|Fire`
  (params (Key :type "Key Structure" :default "AnyKey"))
  ;[1 1 1] Fire Guns
  (:`Pressed`
    (goto _label :!via `Open`))
  (:`Released`
    (goto _label :!via `Close`)))

(fn `UserConstructionScript`)