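; Bullet actor that damages enemies on contact and has a ten-second lifespan.
; Overlap and hit events on its Sphere1 component both check the other actor for the EnemyTargetable interface.
; Matching actors receive engine ApplyDamage, and those that cast to BaseEnemy also get that class's own ApplyDamage call with the same Damage value.
; The actor-level Hit event only prints the other actor's name.
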(event `self.ReceiveHit`
  (params (MyComp :type "PrimitiveComponent Object Reference") (Other :type "Actor Object Reference") (OtherComp :type "PrimitiveComponent Object Reference") (bSelfMoved :type Boolean) (HitLocation :type "Vector Structure") (HitNormal :type "Vector Structure") (NormalImpulse :type "Vector Structure") (Hit :type "HitResult Structure (by ref)"))
  (`KismetSystemLibrary.PrintString` (`KismetSystemLibrary.GetDisplayName` Other)))

(event `self.ReceiveBeginPlay`
  (`self.SetLifeSpan` 10.0))

(event `self.Sphere1.OnComponentBeginOverlap`
  (params (OverlappedComponent :type "PrimitiveComponent Object Reference") (OtherActor :type "Actor Object Reference") (OtherComp :type "PrimitiveComponent Object Reference") (OtherBodyIndex :type Integer) (bFromSweep :type Boolean) (SweepResult :type "HitResult Structure (by ref)"))
  (if (`KismetSystemLibrary.DoesImplementInterface` OtherActor "/Game/Blueprints/Enemies/EnemyTargetable.EnemyTargetable_C")
    (`GameplayStatics.ApplyDamage` OtherActor (`self.Damage`))
    (bind _asbase_enemy (cast `/Game/Blueprints/Enemies/BaseEnemy` OtherActor))
    (`/Game/Blueprints/Enemies/BaseEnemy.ApplyDamage` _asbase_enemy (`self.Damage`))))

(event `self.Sphere1.OnComponentHit`
  (params (HitComponent :type "PrimitiveComponent Object Reference") (OtherActor :type "Actor Object Reference") (OtherComp :type "PrimitiveComponent Object Reference") (NormalImpulse :type "Vector Structure") (Hit :type "HitResult Structure (by ref)"))
  (if (`KismetSystemLibrary.DoesImplementInterface` OtherActor "/Game/Blueprints/Enemies/EnemyTargetable.EnemyTargetable_C")
    (`GameplayStatics.ApplyDamage` OtherActor (`self.Damage`))
    (bind _asbase_enemy (cast `/Game/Blueprints/Enemies/BaseEnemy` OtherActor))
    (`/Game/Blueprints/Enemies/BaseEnemy.ApplyDamage` _asbase_enemy (`self.Damage`))))

(fn `UserConstructionScript`)