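; Homing missile actor that pursues its Target and damages EnemyTargetable actors, self-destructing when the Target is invalid or its lifespan ends.
; Tick sweeps it forward by a fixed per-frame step; after a short delay, a Gate enables lerped look-at steering.
; Sphere1 overlaps and hits apply damage both generically and through BaseEnemy, without destroying the missile.
; A fast looping timer spawns engine-glow emitters as a trail.
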(event `self.ReceiveHit`
  (params (MyComp :type "PrimitiveComponent Object Reference") (Other :type "Actor Object Reference") (OtherComp :type "PrimitiveComponent Object Reference") (bSelfMoved :type Boolean) (HitLocation :type "Vector Structure") (HitNormal :type "Vector Structure") (NormalImpulse :type "Vector Structure") (Hit :type "HitResult Structure (by ref)"))
  (`KismetSystemLibrary.PrintString` (`KismetSystemLibrary.GetDisplayName` Other)))

(event `self.ReceiveTick`
  (params (DeltaSeconds :type "Float (single-precision)"))
  (if (`KismetSystemLibrary.IsValid` (`self.Target`))
    (`|ExecutionSequence`
      (:`then_0`
        (`self.K2_AddActorLocalOffset` (50.0 0.0 0.0) true)
        (`KismetSystemLibrary.Delay` 0.2)
        (`/Engine/EditorBlueprintResources/StandardMacros.DoOnce` false
          (:`Completed`
            (goto _label :!via `Open`))))
      (:`then_1`
        (`/Engine/EditorBlueprintResources/StandardMacros.Gate` true :!label _label
          (:`Exit`
            (if (`KismetSystemLibrary.IsValid` (`self.Target`))
              (`self.K2_SetActorRotation` (`KismetMathLibrary.RLerp` (`self.K2_GetActorRotation`) (`KismetMathLibrary.FindLookAtRotation` (`self.K2_GetActorLocation`) (`self.K2_GetActorLocation` (`self.Target`))) 0.2))
              (else
                (`self.K2_DestroyActor`)))))))
    (else
      (`self.K2_DestroyActor`))))

(event `self.ReceiveBeginPlay`
  (`KismetSystemLibrary.K2_SetTimerDelegate` (delegate `EngineParticles`) 0.01 true)
  (`self.SetLifeSpan` 10.0))

(event `EngineParticles`
  (bind _returnvalue (`GameplayStatics.SpawnEmitterAtLocation` "/Game/Particles/P_EngineGlow.P_EngineGlow" (`SceneComponent.K2_GetComponentLocation` (`self.Sphere`))))
  (`SceneComponent.SetWorldScale3D` _returnvalue (0.25 0.25 0.25)))

(event `self.Sphere1.OnComponentBeginOverlap`
  (params (OverlappedComponent :type "PrimitiveComponent Object Reference") (OtherActor :type "Actor Object Reference") (OtherComp :type "PrimitiveComponent Object Reference") (OtherBodyIndex :type Integer) (bFromSweep :type Boolean) (SweepResult :type "HitResult Structure (by ref)"))
  (if (`KismetSystemLibrary.DoesImplementInterface` OtherActor "/Game/Blueprints/Enemies/EnemyTargetable.EnemyTargetable_C")
    (`GameplayStatics.ApplyDamage` OtherActor (`self.Damage`))
    (bind _asbase_enemy (cast `/Game/Blueprints/Enemies/BaseEnemy` OtherActor))
    (`/Game/Blueprints/Enemies/BaseEnemy.ApplyDamage` _asbase_enemy (`self.Damage`))))

(event `self.Sphere1.OnComponentHit`
  (params (HitComponent :type "PrimitiveComponent Object Reference") (OtherActor :type "Actor Object Reference") (OtherComp :type "PrimitiveComponent Object Reference") (NormalImpulse :type "Vector Structure") (Hit :type "HitResult Structure (by ref)"))
  (if (`KismetSystemLibrary.DoesImplementInterface` OtherActor "/Game/Blueprints/Enemies/EnemyTargetable.EnemyTargetable_C")
    (`GameplayStatics.ApplyDamage` OtherActor (`self.Damage`))
    (bind _asbase_enemy (cast `/Game/Blueprints/Enemies/BaseEnemy` OtherActor))
    (`/Game/Blueprints/Enemies/BaseEnemy.ApplyDamage` _asbase_enemy (`self.Damage`))))

(fn `UserConstructionScript`)