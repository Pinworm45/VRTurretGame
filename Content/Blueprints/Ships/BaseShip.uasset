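; BaseShip is a ship actor that travels along the first SplinePath found in the level and holds references to two child actors as turrets.
; BeginPlay caches the distance of each spline point, then Tick advances the ship by Speed and matches its location and rotation to the spline.
; Nearing the next point increments the segment index and sets WaitTilNextDestination (unread here), or restarts at the path's end.
; MoveToNextSpline is an empty stub.
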(event `self.ReceiveBeginPlay`
  (bind _segmentlocations (`self.SegmentLocations`))
  (set `self.TurretArray` (`|MakeArray` (`self.ChildActor`) (`self.ChildActor1`)))
  (bind _outactors (`GameplayStatics.GetAllActorsOfClass` "/Game/Blueprints/SplinePath.SplinePath_C"))
  (`KismetArrayLibrary.Array_Clear` _segmentlocations)
  (bind _item (`KismetArrayLibrary.Array_Get` _outactors))
  (bind _spline (`/Game/Blueprints/SplinePath.Spline` _item))
  (for _index (range (+ (`SplineComponent.GetNumberOfSplinePoints` _spline) 1))
    (`KismetArrayLibrary.Array_Add` _segmentlocations (`SplineComponent.GetDistanceAlongSplineAtSplinePoint` _spline _index))
    (set `self.SplinePath` _item)))

(event `self.ReceiveTick`
  (params (DeltaSeconds :type "Float (single-precision)"))
  (bind _spline (`/Game/Blueprints/SplinePath.Spline` (`self.SplinePath`)))
  (bind _output_get (set `self.CurrentDistance` (+ (`KismetMathLibrary.FInterpTo` 0.0 (`SplineComponent.GetSplineLength` (`/Game/Blueprints/SplinePath.Spline` (`self.SplinePath`))) DeltaSeconds (`self.Speed`)) (stale _output_get))))
  (`self.K2_SetActorLocationAndRotation` (`SplineComponent.GetLocationAtDistanceAlongSpline` _spline _output_get "World") (`SplineComponent.GetRotationAtDistanceAlongSpline` _spline _output_get "World"))
  (if (< (- (`KismetArrayLibrary.Array_Get` (`self.SegmentLocations`) (+ (`self.CurrSplineNdx`) 1)) (`self.CurrentDistance`)) (`self.DistanceTillNextShift`))
    (`/Engine/EditorBlueprintResources/StandardMacros.CompareInt` (+ (`self.CurrSplineNdx`) 1) (- (`KismetArrayLibrary.Array_Length` (`self.SegmentLocations`)) 1)
      (:`>`
        (set `self.CurrSplineNdx` 0 :!label _label)
        (set `self.CurrentDistance` 0.0))
      (:`==`
        (goto _label))
      (:`<`
        (set `self.CurrSplineNdx` (+ (`self.CurrSplineNdx`) 1))
        (set `self.WaitTilNextDestination` true)))))

(fn `MoveToNextSpline`)

(fn `UserConstructionScript`)