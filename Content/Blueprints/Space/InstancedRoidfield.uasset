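; Blueprint that builds a procedural asteroid field in space around its own origin.
; The construction script adds TotalRoids instances to a single InstancedStaticMesh component instead of creating separate actors or components.
; Each instance gets a random direction and a distance between MinDistance and MaxDistance, forming a spherical shell, plus random rotation and uniform scale.
; Randomization is unseeded, so the layout changes whenever the script reruns.
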(fn `UserConstructionScript`
  (for _ (range 1 (+ (`self.TotalRoids`) 1))
    (`InstancedStaticMeshComponent.AddInstance` (`self.InstancedStaticMesh`) (`KismetMathLibrary.MakeTransform` (* (`KismetMathLibrary.RandomUnitVector`) (`KismetMathLibrary.RandomFloatInRange` (`self.MinDistance`) (`self.MaxDistance`))) (`KismetMathLibrary.RandomRotator` false) (`KismetMathLibrary.Conv_DoubleToVector` (* (`KismetMathLibrary.RandomFloatInRange` (`self.MinScale`) (`self.MaxScale`)) (`self.ScaleMultiplier`)))))))